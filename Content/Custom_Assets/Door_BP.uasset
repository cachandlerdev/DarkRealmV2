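; Door Blueprint with a trigger Box meant to open for the player (Nathan_BP), but as wired it never moves.
; Overlap start opens a flow-control Gate; overlap end closes it only if the same actor casts to both Nathan_BP and key1_BP.
; The Gate's Enter, a "NoKey" message and the DoorAngle timeline that rotates DoorMesh with a creak sound are all in unreached logic.
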(event OnComponentBeginOverlap(Box)
  (params (OverlappedComponent :type Primitive%20Component%20Object%20Reference) (OtherActor :type Actor%20Object%20Reference) (OtherComp :type Primitive%20Component%20Object%20Reference) (OtherBodyIndex :type Integer) (bFromSweep :type Boolean) (SweepResult :type Hit%20Result%20Structure%20%28by%20ref%29))
  (Utilities|Casting|CastToNathan_BP OtherActor)
  ;[1 1 1] Door open/close animation
  (Utilities|FlowControl|Gate true) ; enters at Open
)

(event OnComponentEndOverlap(Box)
  (params (OverlappedComponent :type Primitive%20Component%20Object%20Reference) (OtherActor :type Actor%20Object%20Reference) (OtherComp :type Primitive%20Component%20Object%20Reference) (OtherBodyIndex :type Integer))
  (Utilities|Casting|CastToNathan_BP OtherActor)
  ;[1 1 1] Door open/close animation
  (Utilities|Casting|CastTokey1_BP OtherActor)
  (Utilities|FlowControl|Gate true) ; enters at Close
)

(event Input|ActionEvents|InputActionInteract(Inventory)
  (params (Key :type Key%20Structure :default "None")))

(fn ConstructionScript)