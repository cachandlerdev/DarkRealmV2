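; Lantern path actor that sorts every BP_Lantern in the level along its PlayerPath spline and chains their deactivation.
; On BeginPlay it binds to each lantern's deactivation dispatcher; when one fires, lanterns from the path start through that one are deactivated.
; Ordering samples the spline at DistanceCheck intervals for each lantern's nearest point, then selection-sorts the mapped distances.
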(event Custom|DeactivateLantern
  (params (DeactivatedActor :type BP%20Lantern%20Object%20Reference))
  (bind _points (Variables|Default|GetPoints))
  (bind _returnvalue (Utilities|Array|FindItem _points DeactivatedActor))
  (if (== _returnvalue -1)
    (Development|PrintString "SOMETHING HAS GONE HORRIBLY WRONG")
    (else
      (for _index (range 0 _returnvalue)
        (bind _asbplantern (Utilities|Casting|CastToBP_Lantern (Utilities|Array|Get(acopy) (Variables|Default|GetPoints) _index)))
        (Default|Deactivate _asbplantern)))))

(event EventBeginPlay
  (bind _outactors (Actor|GetAllActorsOfClass "/Game/Blueprints/BP_Lantern.BP_Lantern_C"))
  (bind _orderedpoints (CallFunction|OrderActorstoDistanceAlongSpline _outactors (Variables|Default|GetPlayerPath)))
  (bind _output_get (Variables|Default|SetPoints _orderedpoints))
  (for _array_element _output_get
    (bind _asbplantern (Utilities|Casting|CastToBP_Lantern _array_element))
    (EventDispatchers|BindEventtoOnDeactivatedDispatch _asbplantern (delegate Custom|DeactivateLantern))))

(fn ConstructionScript)

(fn OrderActorstoDistanceAlongSpline
  (params (ActorsToOrder :type Array%20of%20Actor%20Object%20References) (Spline :type Spline%20Component%20Object%20Reference))
  ;[1 1 1] Get Distances
  (for _array_element ActorsToOrder
    (LocalVariables|SetCurrentActor _array_element)
    (LocalVariables|SetCurrentShortestDistanceAlongSpline 0.0)
    (LocalVariables|SetCurrentShortestDistance (Math|Vector|Distance(Vector) (Transformation|GetActorLocation (LocalVariables|GetCurrentActor)) (Spline|GetLocationatDistanceAlongSpline Spline 0.0 "World")))
    (for _index (range 1 (Math|Float|Truncate (/ (Spline|GetSplineLength (Variables|Default|GetPlayerPath)) (LocalVariables|GetDistanceCheck))))
      (if (< (Math|Vector|Distance(Vector) (Transformation|GetActorLocation (LocalVariables|GetCurrentActor)) (Spline|GetLocationatDistanceAlongSpline Spline (* _index (LocalVariables|GetDistanceCheck)) "World")) (LocalVariables|GetCurrentShortestDistance))
        (LocalVariables|SetCurrentShortestDistanceAlongSpline (* _index (LocalVariables|GetDistanceCheck)))
        (LocalVariables|SetCurrentShortestDistance (Math|Vector|Distance(Vector) (Transformation|GetActorLocation (LocalVariables|GetCurrentActor)) (Spline|GetLocationatDistanceAlongSpline Spline (* _index (LocalVariables|GetDistanceCheck)) "World")))))
    (Utilities|Map|Add (LocalVariables|GetActorsToDistances) (LocalVariables|GetCurrentActor) (LocalVariables|GetCurrentShortestDistanceAlongSpline)))
  (while (> (Utilities|Map|Length (LocalVariables|GetActorsToDistances)) 0)
    (bind _keys (Utilities|Map|Keys (LocalVariables|GetActorsToDistances)))
    (for (_array_element_2 _array_index) _keys
      (if (== _array_index 0)
        (LocalVariables|SetCurrentActor _array_element_2 :!label _label)
        (LocalVariables|SetCurrentShortestDistanceAlongSpline (.Value (Utilities|Map|Find (LocalVariables|GetActorsToDistances) _array_element_2)))
        (elif (< (.Value (Utilities|Map|Find (LocalVariables|GetActorsToDistances) _array_element_2)) (LocalVariables|GetCurrentShortestDistanceAlongSpline))
          (goto _label))))
    (Utilities|Array|Add (LocalVariables|GetOrderedActors) (LocalVariables|GetCurrentActor))
    (Utilities|Map|Remove (LocalVariables|GetActorsToDistances) (LocalVariables|GetCurrentActor)))
  (return (LocalVariables|GetOrderedActors)))