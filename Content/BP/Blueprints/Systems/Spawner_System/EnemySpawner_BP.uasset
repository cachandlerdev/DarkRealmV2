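; Enemy spawner actor that keeps a single random enemy from its class list at its own transform, spawning on BeginPlay.
; Each enemy receives a reference to the spawner, whose Respawn event clears it and spawns again after a delay, unless that delay is zero.
; EnemyNPC spawns get a custom name and level, plus an optional weapon and shield loadout with AI attack timing and range set by weapon type.
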(event EventBeginPlay
  (CallFunction|AttempttoSpawn))

(event EventRespawn
  (Variables|Default|SetCurrentEnemy 0)
  (if (!= (Variables|CustomizableParameters|GetRespawnDelay) 0.0)
    (Utilities|FlowControl|Delay (Variables|CustomizableParameters|GetRespawnDelay))
    (CallFunction|AttempttoSpawn)))

(fn ConstructionScript)

(fn AttempttoSpawn
  (Utilities|IsValid (Variables|Default|GetCurrentEnemy)
    (:Is%20Not%20Valid
      (CallFunction|SpawnEnemy))))

(fn SpawnEnemy
  (bind _enemiestospawn (Variables|CustomizableParameters|GetEnemiesToSpawn))
  (bind _returnvalue (Game|SpawnActorfromClass (Utilities|Array|Get(acopy) _enemiestospawn (Math|Random|RandomIntegerinRange 0 (Utilities|Array|LastIndex _enemiestospawn))) (Math|Transform|MakeTransform (Transformation|GetActorLocation) (Transformation|GetActorRotation)) "Undefined" 0 self 0))
  (bind _output_get (Variables|Default|SetCurrentEnemy _returnvalue))
  (Utilities|Casting|CastToEnemyNPC _output_get)
  (CallFunction|CustomStats))

(fn CustomStats
  (bind _asenemy_npc (Utilities|Casting|CastToEnemyNPC (Variables|Default|GetCurrentEnemy)))
  (Variables|/Game/BP/Blueprints/Systems/Stats_System/Stats_Component.Stats_Component_C|SetName (Variables|/Game/BP/Blueprints/AI/EnemyNPC/EnemyNPC.EnemyNPC_C|GetStats_Component _asenemy_npc) (Variables|CustomizableStats|GetEnemy%20Name))
  (Variables|/Game/BP/Blueprints/Systems/Stats_System/Stats_Component.Stats_Component_C|SetCurrent%20Level (Variables|/Game/BP/Blueprints/AI/EnemyNPC/EnemyNPC.EnemyNPC_C|GetStats_Component _asenemy_npc) (Variables|CustomizableStats|GetEnemy%20Level))
  (if (Variables|CustomizableParameters|GetUseCustomLoadout)
    (switch Utilities|FlowControl|Switch|SwitchonWeapon_Type (Variables|CustomizableStats|GetPrimary%20Weapon%20Type)
      (:NewEnumerator0
        (Variables|CustomizableStats|SetAI%20Delay%20Time 0.85)
        (Variables|CustomizableStats|SetAI%20Melee%20Range 2.5e+02))
      (:NewEnumerator9
        (Variables|CustomizableStats|SetAI%20Delay%20Time 0.85)
        (Variables|CustomizableStats|SetAI%20Melee%20Range 3e+02))
      (:NewEnumerator2
        (Variables|CustomizableStats|SetAI%20Delay%20Time 0.85)
        (Variables|CustomizableStats|SetAI%20Melee%20Range 1e+02))
      (:NewEnumerator1
        (Variables|CustomizableStats|SetAI%20Delay%20Time 1.3)
        (Variables|CustomizableStats|SetAI%20Melee%20Range 2.5e+02))
      (:NewEnumerator5
        (Variables|CustomizableStats|SetAI%20Delay%20Time 1.3)
        (Variables|CustomizableStats|SetAI%20Melee%20Range 2.5e+02))
      (:NewEnumerator10
        (Variables|CustomizableStats|SetAI%20Delay%20Time 0.6)
        (Variables|CustomizableStats|SetAI%20Melee%20Range 1.5e+02)))
    (Utilities|Map|Add (Variables|/Game/BP/Blueprints/Systems/Inventory_System/Equipment_Inventory/Equipment_Inventory_Component.Equipment_Inventory_Component_C|GetEquipped_Weapons (Variables|/Game/BP/Blueprints/AI/EnemyNPC/EnemyNPC.EnemyNPC_C|GetEquipment_Inventory_Component _asenemy_npc)) "NewEnumerator0" (Utilities|Struct|MakeWeapon_Data 0 "Custom" "Custom" (Variables|CustomizableStats|GetPrimary%20Weapon%20Type) "NewEnumerator0" "NewEnumerator0" (Variables|CustomizableStats|GetWeapon%20Damage) 0.0 0.0 0 (Variables|CustomizableStats|GetWeapon%20Mesh) (Variables|CustomizableStats|GetAI%20Delay%20Time) (Variables|CustomizableStats|GetAI%20Melee%20Range)))
    (Utilities|Map|Add (Variables|/Game/BP/Blueprints/Systems/Inventory_System/Equipment_Inventory/Equipment_Inventory_Component.Equipment_Inventory_Component_C|GetEquipped_Weapons (Variables|/Game/BP/Blueprints/AI/EnemyNPC/EnemyNPC.EnemyNPC_C|GetEquipment_Inventory_Component _asenemy_npc)) "NewEnumerator1" (Utilities|Struct|MakeWeapon_Data 0 "Custom" "Custom" "NewEnumerator8" "NewEnumerator1" "NewEnumerator0" 0.0 0.0 (Variables|CustomizableStats|GetShield%20Defense) 0 (Variables|CustomizableStats|GetShield%20Mesh)))
    (bind _asenemy_npc_2 (Utilities|Casting|CastToEnemyNPC (Variables|Default|GetCurrentEnemy)))
    (Default|RefreshStats _asenemy_npc_2)))