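; Item spawner actor that spawns one weighted-random item at its own location on BeginPlay.
; Its Respawn event clears the current item and, if a delay is set, spawns a replacement afterward.
; Candidate classes are sorted into Common, Uncommon, Rare and Epic pools by reading rarity from class defaults.
; A twenty-sided weighted roll picks the tier, rerolling on empty pools with some range narrowing, then picks a random class from that pool.
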(event EventBeginPlay
  (CallFunction|AttempttoSpawn))

(event EventRespawn
  (Variables|Default|SetCurrentItem 0)
  (if (!= (Variables|Default|GetRespawnDelay) 0.0)
    (Utilities|FlowControl|Delay (Variables|Default|GetRespawnDelay))
    (CallFunction|AttempttoSpawn)))

(fn ConstructionScript)

(fn AttempttoSpawn
  (Utilities|IsValid (Variables|Default|GetCurrentItem)
    (:Is%20Not%20Valid
      (CallFunction|SpawnItem))))

(fn SpawnItem
  (bind _returnvalue (Game|SpawnActorfromClass (CallFunction|DetermineItemtoSpawn) (Math|Transform|MakeTransform (Transformation|GetActorLocation) (Transformation|GetActorRotation)) "AdjustIfPossibleButAlwaysSpawn" self 0))
  (Variables|Default|SetCurrentItem _returnvalue))

(fn DetermineItemtoSpawn
  (for _array_element (Variables|Default|GetItemsToSpawn)
    (if (Utilities|IsValidClass _array_element)
      (switch Utilities|FlowControl|Switch|SwitchonRarity (.Rarity (Utilities|Struct|BreakItem_Structure (.ItemStructure (Utilities|GetClassDefaults _array_element))))
        (:NewEnumerator0
          (Utilities|Array|AddUnique (LocalVariables|GetCommonItems) _array_element))
        (:NewEnumerator1
          (Utilities|Array|AddUnique (LocalVariables|GetUncommonItems) _array_element))
        (:NewEnumerator2
          (Utilities|Array|AddUnique (LocalVariables|GetRareItems) _array_element))
        (:NewEnumerator3
          (Utilities|Array|AddUnique (LocalVariables|GetEpicItems) _array_element)))))
  (bind _item (CallFunction|RarityAlgorithm (LocalVariables|GetCommonItems) (LocalVariables|GetUncommonItems) (LocalVariables|GetRareItems) (LocalVariables|GetEpicItems) (>= (Utilities|Array|Length (LocalVariables|GetCommonItems)) 1) (>= (Utilities|Array|Length (LocalVariables|GetUncommonItems)) 1) (>= (Utilities|Array|Length (LocalVariables|GetRareItems)) 1) (>= (Utilities|Array|Length (LocalVariables|GetEpicItems)) 1)))
  (return _item))

(fn RarityAlgorithm
  (params (Common%20Items :type Array%20of%20Item%20Class%20References) (Uncommon%20Items :type Array%20of%20Item%20Class%20References) (Rare%20Items :type Array%20of%20Item%20Class%20References) (Epic%20Items :type Array%20of%20Item%20Class%20References) (SpawnCommon :type Boolean) (SpawnUncommon :type Boolean) (SpawnRare :type Boolean) (SpawnEpic :type Boolean))
  (while (LocalVariables|GetKeepLooping)
    (if (Math|Boolean|ORBoolean (LocalVariables|GetCheckedCommonAlready) (LocalVariables|GetCheckedUncommonAlready) (LocalVariables|GetCheckedRareAlready) (LocalVariables|GetCheckedEpicAlready))
      (Utilities|FlowControl|Sequence
        (:then_0
          (Utilities|FlowControl|DoOnce false
            (:Completed
              ;[1 1 1] Reduce range based on available rarity
              (Utilities|FlowControl|Sequence
                (:then_0
                  (if (LocalVariables|GetCheckedCommonAlready)
                    (LocalVariables|SetMinimum%20Number 10)))
                (:then_1
                  (if (LocalVariables|GetCheckedEpicAlready)
                    (LocalVariables|SetMaximum%20Number 19)))
                (:then_2
                  (if (and (LocalVariables|GetCheckedCommonAlready) (LocalVariables|GetCheckedUncommonAlready))
                    (LocalVariables|SetMinimum%20Number 16)))
                (:then_3
                  (if (and (LocalVariables|GetCheckedRareAlready) (LocalVariables|GetCheckedEpicAlready))
                    (LocalVariables|SetMaximum%20Number 15)))
                (:then_4
                  (bind _output_get (LocalVariables|SetRandomNumber (Math|Random|RandomIntegerinRange (LocalVariables|GetMinimum%20Number) (LocalVariables|GetMaximum%20Number)) :!label _label))
                  (Utilities|FlowControl|Sequence
                    (:then_0
                      ;[1 1 1] Common 50% (1-10)
                      (if (Math|Integer|InRange(Integer) _output_get 1 10)
                        (if SpawnCommon
                          (LocalVariables|SetItemClass (Utilities|Array|Get(acopy) Common%20Items (Math|Random|RandomIntegerinRange 0 (- (Utilities|Array|Length Common%20Items) 1))))
                          (LocalVariables|SetKeepLooping false)
                          (else
                            (LocalVariables|SetCheckedCommonAlready true)))))
                    (:then_1
                      ;[1 1 1] Uncommon 30% (11-16)
                      (if (Math|Integer|InRange(Integer) _output_get 11 16)
                        (if SpawnUncommon
                          (LocalVariables|SetItemClass (Utilities|Array|Get(acopy) Uncommon%20Items (Math|Random|RandomIntegerinRange 0 (- (Utilities|Array|Length Uncommon%20Items) 1))))
                          (LocalVariables|SetKeepLooping false)
                          (else
                            (LocalVariables|SetCheckedUncommonAlready true)))))
                    (:then_2
                      ;[1 1 1] Rare 15% (17-19)
                      (if (Math|Integer|InRange(Integer) _output_get 17 19)
                        (if SpawnRare
                          (LocalVariables|SetItemClass (Utilities|Array|Get(acopy) Rare%20Items (Math|Random|RandomIntegerinRange 0 (- (Utilities|Array|Length Rare%20Items) 1))))
                          (LocalVariables|SetKeepLooping false)
                          (else
                            (LocalVariables|SetCheckedRareAlready true)))))
                    (:then_3
                      ;[1 1 1] Epic 5% (20)
                      (if (Math|Integer|InRange(Integer) _output_get 20 20)
                        (if SpawnEpic
                          (LocalVariables|SetItemClass (Utilities|Array|Get(acopy) Epic%20Items (Math|Random|RandomIntegerinRange 0 (- (Utilities|Array|Length Epic%20Items) 1))))
                          (LocalVariables|SetKeepLooping false)
                          (else
                            (LocalVariables|SetCheckedEpicAlready true)))))))))))
        (:then_1
          (goto _label)))
      (else
        (goto _label))))
  (return (LocalVariables|GetItemClass)))