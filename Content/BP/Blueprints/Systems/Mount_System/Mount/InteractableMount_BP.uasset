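; InteractableMount_BP is an interactable mount that puts the player in control of a Griffon_BP when used.
; On Interact, it spawns the griffon slightly above its own location with matching rotation and scale, then possesses it.
; It also hides the player's HUD, cancels sprint, hides and teleports the character to the world origin, and hides itself.
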(event EventBeginPlay
  (bind _asthird_person_character (Utilities|Casting|CastToThirdPersonCharacter (Game|GetPlayerCharacter 0)))
  (Variables|Default|SetPlayerCharacter _asthird_person_character))

(event EventInteract
  (params (Interactor :type Actor%20Object%20Reference))
  (bind _returnvalue (Game|GetPlayerCharacter 0))
  (bind _returnvalue_2 (Transformation|GetActorTransform))
  ;[1 1 1] Interact
  (bind _returnvalue_3 (Game|SpawnActorfromClass "/Game/FlyingBP/Blueprints/Griffon_BP.Griffon_BP_C" (Math|Transform|MakeTransform (CallFunction|GetValidLocation) (.rotation _returnvalue_2) (.scale _returnvalue_2)) "Undefined" 0 0))
  (Widget|SetVisibility (Variables|/Game/BP/Blueprints/Characters/PlayerCharacter/ThirdPersonCharacter.ThirdPersonCharacter_C|GetHealthAndXP_UI (Variables|Default|GetPlayerCharacter)) "Hidden")
  (Rendering|SetActorHiddenInGame _returnvalue true)
  (Transformation|Teleport _returnvalue "0, 0, 0" "0, 0, 0")
  (Variables|/Game/BP/Blueprints/Characters/PlayerCharacter/ThirdPersonCharacter.ThirdPersonCharacter_C|SetCancelSprint? (Variables|Default|GetPlayerCharacter) true)
  (Rendering|SetActorHiddenInGame self true)
  (Pawn|Possess (Game|GetPlayerController 0) _returnvalue_3))

(fn ConstructionScript)

(fn GetValidLocation
  (bind _returnvalue (Transformation|GetActorLocation))
  (return (Math|Vector|MakeVector (.x _returnvalue) (.y _returnvalue) (+ (.z _returnvalue) 145.0))))